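; Ranged door actor that slides along the X axis as soon as play begins, then destroys itself.
; BeginPlay records the start location and runs a timeline that lerps the actor to a fixed X coordinate, keeping Y and Z, without sweeping.
; A hit on the Bottom component spawns a sound at the actor's location.
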(event `self.Bottom.OnComponentHit`
  (params (HitComponent :type "PrimitiveComponent Object Reference") (OtherActor :type "Actor Object Reference") (OtherComp :type "PrimitiveComponent Object Reference") (NormalImpulse :type "Vector Structure") (Hit :type "HitResult Structure (by ref)"))
  (`GameplayStatics.SpawnSoundAtLocation` "/Game/Bluebrints/Sound2.Sound2" (`self.K2_GetActorLocation`) (struct) 1.0 1.0 0.0 null null))

(event `self.ReceiveBeginPlay`
  (bind (_returnvalue_x _returnvalue_y _returnvalue_z) (`KismetMathLibrary.BreakVector` (`self.K2_GetActorLocation`)))
  (set `self.StartPoint` (`KismetMathLibrary.MakeVector` _returnvalue_x _returnvalue_y _returnvalue_z))
  (set `self.EndPoint` (`KismetMathLibrary.MakeVector` 1400.0 _returnvalue_y _returnvalue_z))
  (bind (_direction _movement) (`Timeline|Timeline_0` :!via `PlayFromStart`)
    (:`Update`
      (`self.K2_SetActorRelativeLocation` (`KismetMathLibrary.VLerp` (`self.StartPoint`) (`self.EndPoint`) _movement)))
    (:`Finished`
      (`self.K2_DestroyActor`))))

(fn `UserConstructionScript`)
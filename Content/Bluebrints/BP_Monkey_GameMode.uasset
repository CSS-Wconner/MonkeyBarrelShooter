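; BP_Monkey_GameMode is a game mode that tracks score, remaining targets and elapsed time for a target-based level.
; UpdateTargets decrements the available target count, while AddPoints increases the player score and Tick accumulates total time.
; AddPoints plays HighScore when the score equals a hardcoded threshold, and adds the HUD_Button widget to the viewport when it equals the level-one target count.
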(event `UpdateTargets`
  ;[1 1 1] Update available targets variable
  (set `self.Available_Targets` (- (`self.Available_Targets`) 1.0)))

(event `AddPoints`
  (params (`Add Score Point` :type Integer))
  ;[1 1 1] Add Points to Score Variable
  (bind _output_get (set `self.Player_Score` (+ `Add Score Point` (`self.Player_Score`))))
  (if (== 20 _output_get)
    (`AudioComponent.Play` (`self.HighScore`) 0.0))
  (if (== _output_get (`self.LevelOne_Targets`))
    (bind _returnvalue (`|CreateWidget` "/Game/Bluebrints/HUD_Button.HUD_Button_C"))
    (`UserWidget.AddToViewport` _returnvalue 0)))

(event `self.ReceiveTick`
  (params (DeltaSeconds :type "Float (single-precision)"))
  ;[1 1 1] Set Total_Time using Delta Time
  (set `self.Total_Time` (+ (`self.Total_Time`) DeltaSeconds)))

(fn `UserConstructionScript`)
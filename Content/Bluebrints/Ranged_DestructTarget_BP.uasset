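; Ranged_DestructTarget_BP is a moving target actor that slides along the X axis and removes itself when it reaches the end of its path.
; On BeginPlay it records its location and plays the Movement timeline, lerping its relative location toward a fixed X coordinate while keeping Y and Z.
; The actor destroys itself when the timeline finishes.
; A hit on the Targetbody component plays a sound at the actor's location.
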(event `self.ReceiveBeginPlay`
  (bind (_returnvalue_x _returnvalue_y _returnvalue_z) (`KismetMathLibrary.BreakVector` (`self.K2_GetActorLocation`)))
  (set `self.StartPoint` (`KismetMathLibrary.MakeVector` _returnvalue_x _returnvalue_y _returnvalue_z))
  (set `self.EndPoint` (`KismetMathLibrary.MakeVector` -1400.0 _returnvalue_y _returnvalue_z))
  (bind (_direction _movement) (`Timeline|Movement` :!via `PlayFromStart`)
    (:`Update`
      (`self.K2_SetActorRelativeLocation` (`KismetMathLibrary.VLerp` (`self.StartPoint`) (`self.EndPoint`) _movement)))
    (:`Finished`
      (`self.K2_DestroyActor`))))

(event `self.Targetbody.OnComponentHit`
  (params (HitComponent :type "PrimitiveComponent Object Reference") (OtherActor :type "Actor Object Reference") (OtherComp :type "PrimitiveComponent Object Reference") (NormalImpulse :type "Vector Structure") (Hit :type "HitResult Structure (by ref)"))
  (`GameplayStatics.SpawnSoundAtLocation` "/Game/Bluebrints/Sound1.Sound1" (`self.K2_GetActorLocation`) (struct) 1.0 1.0 0.0 null null))

(fn `UserConstructionScript`)
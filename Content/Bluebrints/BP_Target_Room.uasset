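; BP_Target_Room is a room trigger that reveals its targets when the player enters and opens the door to the next room once all are destroyed.
; At BeginPlay it caches the BP_Target_Basic actors overlapping its Box, then calls RevealTarget on each when a FirstPersonCharacter overlaps.
; Tick polls the cached references with IsValid, calls OpenDoor when none remain valid, then disables its own tick.
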(event `self.ReceiveBeginPlay`
  ;[1 1 1] Define Targets in Room
  (set `self.TargetsInRoom` (`PrimitiveComponent.GetOverlappingActors` (`self.Box`) "/Game/Bluebrints/BP_Target_Basic.BP_Target_Basic_C")))

(event `self.Box.OnComponentBeginOverlap`
  (params (OverlappedComponent :type "PrimitiveComponent Object Reference") (OtherActor :type "Actor Object Reference") (OtherComp :type "PrimitiveComponent Object Reference") (OtherBodyIndex :type Integer) (bFromSweep :type Boolean) (SweepResult :type "HitResult Structure (by ref)"))
  ;[1 1 1] Reveal Targets when Player Enters Room
  (cast `/Game/FirstPersonBP/Blueprints/FirstPersonCharacter` OtherActor)
  (for _array_element (`self.TargetsInRoom`)
    (`/Engine/EditorBlueprintResources/StandardMacros.IsValid` _array_element
      (:`Is Valid`
        (bind _asbp_target_basic (cast `/Game/Bluebrints/BP_Target_Basic` _array_element))
        (`/Game/Bluebrints/BP_Target_Basic.RevealTarget` _asbp_target_basic)))))

(event `self.ReceiveTick`
  (params (DeltaSeconds :type "Float (single-precision)"))
  ;[1 1 1] Check Status of Targets & Open Door when all are destroyed.
  (set `self.AllTargetDestroyed?` true)
  (for _array_element (`self.TargetsInRoom`)
    (`/Engine/EditorBlueprintResources/StandardMacros.IsValid` _array_element
      (:`Is Valid`
        (set `self.AllTargetDestroyed?` false))))
  (if (`self.AllTargetDestroyed?`)
    (`/Game/Bluebrints/BP_Door.OpenDoor` (`self.DoortoNextRoom`))
    (`self.SetActorTickEnabled` false)))

(fn `UserConstructionScript`)
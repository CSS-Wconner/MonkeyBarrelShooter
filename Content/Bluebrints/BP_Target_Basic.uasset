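; BP_Target_Basic is a shootable target actor that can only be destroyed once it has been revealed.
; Projectile hits on TargetHitBox call TargetHit when TargetRevealed is set, spawning an explosion effect and sound before destroying the actor.
; The RevealTarget event sets that flag, and BeginPlay applies a configurable starting roll while keeping pitch and yaw.
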(event `TargetHit`
  (bind _returnvalue (`self.K2_GetActorLocation`))
  ;[1 1 1] Target Hit generates explosion & destroys target
  (`GameplayStatics.SpawnEmitterAtLocation` "/Game/StarterContent/Particles/P_Explosion.P_Explosion" _returnvalue (struct) (3.0 3.0 3.0))
  (`GameplayStatics.PlaySoundAtLocation` "/Game/StarterContent/Audio/Explosion01.Explosion01" _returnvalue (struct) 1.0 1.0 0.0 null null null)
  (`self.K2_DestroyActor`))

(event `self.TargetHitBox.OnComponentHit`
  (params (HitComponent :type "PrimitiveComponent Object Reference") (OtherActor :type "Actor Object Reference") (OtherComp :type "PrimitiveComponent Object Reference") (NormalImpulse :type "Vector Structure") (Hit :type "HitResult Structure (by ref)"))
  ;[1 1 1] Unrevealed Targets may not be hit
  (cast `/Game/FirstPersonBP/Blueprints/FirstPersonProjectile` OtherActor)
  (if (`self.TargetRevealed`)
    (`self.TargetHit`)))

(event `self.ReceiveBeginPlay`
  (bind (_returnvalue_roll _returnvalue_pitch _returnvalue_yaw) (`KismetMathLibrary.BreakRotator` (`self.K2_GetActorRotation`)))
  ;[1 1 1] All Targets have Rotation Function
  (`self.K2_SetActorRotation` (`KismetMathLibrary.MakeRotator` (`self.Start_X_Rotation`) _returnvalue_pitch _returnvalue_yaw)))

(event `RevealTarget`
  ;[1 1 1] Inherited Call to Reveal Targets
  (set `self.TargetRevealed` true))

(fn `UserConstructionScript`)
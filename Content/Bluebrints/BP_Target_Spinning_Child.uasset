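; BP_Target_Spinning_Child is a child target Blueprint that spins when hit before running the parent's destruction logic.
; TargetHit sets a HasBeenHit flag and waits one second before calling the parent implementation, delaying destruction so the animation can play.
; While the flag is set, Tick rotates TargetHitBox rapidly around its local yaw axis, scaled by delta time.
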(event `self.TargetHit`
  ;[1 1 1] Target Destruction will be delayed for spinning animation.
  (set `self.HasBeenHit` true)
  (`KismetSystemLibrary.Delay` 1.0)
  (`parent.TargetHit`))

(event `self.ReceiveTick`
  (params (DeltaSeconds :type "Float (single-precision)"))
  ;[1 1 1] Target will spin when hit.
  (if (`self.HasBeenHit`)
    (`SceneComponent.K2_AddLocalRotation` (`self.TargetHitBox`) (`KismetMathLibrary.MakeRotator` 0.0 0.0 (* DeltaSeconds 2000.0)) false false)))

(fn `UserConstructionScript`
  (`parent.UserConstructionScript`))